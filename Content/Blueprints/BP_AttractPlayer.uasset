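; BP_AttractPlayer is an actor that fires its PlayerOwner's projectile type at a given target.
; Its Fire event waits for FireRate, checks that the target is still valid, then has PlayerOwner spawn the projectile at ProjectileSpawn.
; The shot is rotated toward the target's BP_Target component rather than the actor's origin.
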(event EventBeginPlay
  (|CallParentFunction))

(event Collision|EventActorBeginOverlap
  (params (OtherActor :type Actor%20Object%20Reference)))

(event EventTick
  (params (DeltaSeconds :type Float%20%28single-precision%29))
  (|CallParentFunction DeltaSeconds) ; This node is disabled and will not be called.\nDrag off pins to build functionality.
)

(event EventFire
  (params (Fire%20At :type Actor%20Object%20Reference))
  (bind _projectile_spawn (Variables|Default|GetProjectile%20Spawn))
  (bind _returnvalue (Transformation|GetWorldLocation _projectile_spawn))
  (Utilities|FlowControl|Delay (Variables|Default|GetFire%20Rate))
  (Utilities|IsValid Fire%20At
    (:Is%20Valid
      (Class|ItemOwner|SpawnProjectile (Variables|Default|GetPlayerOwner) (Variables|/Script/A1GameStudioProject.ItemOwner|GetProjectileType (Variables|Default|GetPlayerOwner)) (Math|Transform|MakeTransform _returnvalue (Math|Rotator|FindLookatRotation _returnvalue (Transformation|GetWorldLocation (Actor|GetComponentbyClass Fire%20At "/Game/Blueprints/Enemies/BP_Target.BP_Target_C"))))))))

(fn ConstructionScript
  (|CallParentFunction))