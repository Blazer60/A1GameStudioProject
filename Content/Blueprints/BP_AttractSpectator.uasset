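; Spectator pawn that follows a BP_AttractPlayer, apparently for an attract mode, while allowing free look.
; On BeginPlay it spawns the BP_AttractPlayer from its root component's relative transform and stores it as the target.
; Each tick it snaps its location to that target without sweeping, leaving rotation to the LookUp and Turn axes, which drive controller pitch and yaw.
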(event EventBeginPlay
  (bind _returnvalue (Game|SpawnActorfromClass "/Game/Blueprints/BP_AttractPlayer.BP_AttractPlayer_C" (Transformation|GetRelativeTransform (Variables|Default|GetDefaultSceneRoot)) "Undefined" 0 0))
  (Variables|Default|SetTarget _returnvalue))

(event Collision|EventActorBeginOverlap
  (params (OtherActor :type Actor%20Object%20Reference)))

(event EventTick
  (params (DeltaSeconds :type Float%20%28single-precision%29))
  (Transformation|SetActorLocation (Transformation|GetActorLocation (Variables|Default|GetTarget)) false false))

(event Input|AxisEvents|InputAxisLookUp
  (params (AxisValue :type Float%20%28single-precision%29))
  (Pawn|Input|AddControllerPitchInput AxisValue))

(event Input|AxisEvents|InputAxisTurn
  (params (AxisValue :type Float%20%28single-precision%29))
  (Pawn|Input|AddControllerYawInput AxisValue))

(fn ConstructionScript)