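; Angler enemy Blueprint, a child class that customizes firing and hurt reactions on top of its parent.
; Fire waits through a fixed delay before passing the target to the parent's Fire.
; BeginPlay binds OnHurt to HurtCallback without calling the parent BeginPlay.
; OnHurt calls PlaySoundAtLocation at the world origin with no sound set, ignoring the attacker and damage.
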(event Custom|On%20Hurt
  (params (HurtBy :type Item%20Owner%20Object%20Reference) (Damage :type Float%20%28single-precision%29))
  (Audio|PlaySoundatLocation 0 "0, 0, 0" "0, 0, 0" 1.0 1.0 0.0 0 0 0))

(event EventBeginPlay
  (Class|HurtCallback|Subscribe (Variables|Default|GetHurtCallback) (delegate Custom|On%20Hurt)))

(event Collision|EventActorBeginOverlap
  (params (OtherActor :type Actor%20Object%20Reference))
  (|CallParentFunction OtherActor) ; This node is disabled and will not be called.\nDrag off pins to build functionality.
)

(event EventTick
  (params (DeltaSeconds :type Float%20%28single-precision%29))
  (|CallParentFunction DeltaSeconds) ; This node is disabled and will not be called.\nDrag off pins to build functionality.
)

(event EventFire
  (params (Fire%20At :type Actor%20Object%20Reference))
  (Utilities|FlowControl|Delay 5.0)
  (|CallParentFunction Fire%20At))

(fn ConstructionScript
  (|CallParentFunction))