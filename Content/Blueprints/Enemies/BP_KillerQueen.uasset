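; BP_KillerQueen is a hovering actor that faces the player and can detonate itself through a Fire event.
; Each tick, its Point component bobs on a sine wave and rotates toward the player pawn.
; Fire spawns BP_Expansion, waits briefly, has ItemOwner spawn its projectile type, then destroys the actor.
; Separately, player overlap with SoundCollision plays snap and delayed boom sounds at the world origin.
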(event OnComponentBeginOverlap(SoundCollision)
  (params (OverlappedComponent :type Primitive%20Component%20Object%20Reference) (OtherActor :type Actor%20Object%20Reference) (OtherComp :type Primitive%20Component%20Object%20Reference) (OtherBodyIndex :type Integer) (bFromSweep :type Boolean) (SweepResult :type Hit%20Result%20Structure%20%28by%20ref%29))
  (Utilities|Casting|CastToBP_MainPlayer OtherActor)
  (Audio|PlaySoundatLocation "/Game/Users/Lauren/Audio/Enemies/Killerqueen_Snap.Killerqueen_Snap" "0, 0, 0" "0, 0, 0" 1.0 1.0 0.0 0 0 0)
  (Utilities|FlowControl|Delay 0.3)
  (Audio|PlaySoundatLocation "/Game/Users/Lauren/Audio/Enemies/Killerqueen_BOOM.Killerqueen_BOOM" "0, 0, 0" "0, 0, 0" 1.0 1.0 0.0 0 0 0))

(event Custom|Face%20Player
  ;[0 0 0] Look at target
  (Transformation|SetWorldRotation (Variables|Default|GetPoint) (Math|Interpolation|RInterpTo (Transformation|GetActorRotation) (Math|Rotator|FindLookatRotation (Transformation|GetWorldLocation (Variables|Default|GetPoint)) (Transformation|GetActorLocation (Variables|Default|GetTracking))) (Utilities|Time|GetWorldDeltaSeconds) 2e+02) false false))

(event EventFire
  (params (Fire%20At :type Actor%20Object%20Reference))
  (bind _capsulecomponent (Variables|Default|GetCapsuleComponent))
  (bind _returnvalue (Transformation|GetWorldLocation _capsulecomponent))
  (bind _returnvalue_2 (Math|Transform|MakeTransform _returnvalue))
  (Game|SpawnActorfromClass "/Game/Blueprints/Props/BP_Expansion.BP_Expansion_C" _returnvalue_2 "Undefined" 0 0)
  (Utilities|FlowControl|Delay 1.0)
  (Class|ItemOwner|SpawnProjectile (Variables|Default|GetItemOwner) (Variables|/Script/A1GameStudioProject.ItemOwner|GetProjectileType (Variables|Default|GetItemOwner)) _returnvalue_2)
  (Actor|DestroyActor))

(event EventTick
  (params (DeltaSeconds :type Float%20%28single-precision%29))
  (bind _relativelocation (Variables|Default|GetRelativeLocation))
  (CallFunction|FacePlayer)
  (Transformation|SetRelativeLocation (Variables|Default|GetPoint) (Math|Vector|MakeVector (.x _relativelocation) (.y _relativelocation) (+ (.z _relativelocation) (* (Math|Trig|Sin(Degrees) (* (Actor|GetGameTimeSinceCreation) (Variables|Default|GetSpeed))) (Variables|Default|GetDistance)))) false false))

(event EventBeginPlay
  (Variables|Default|SetRelativeLocation (Variables|/Script/Engine.SceneComponent|GetRelativeLocation (Variables|Default|GetPoint)))
  (Variables|Default|SetTracking (Game|Player|GetPlayerPawn 0)))

(fn ConstructionScript
  (|CallParentFunction))