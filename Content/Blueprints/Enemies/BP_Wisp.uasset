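; BP_Wisp is an enemy that takes a random head mesh at BeginPlay and can fire projectiles at a target actor.
; Its Move event finds a path to a random nearby navmesh point and issues a simple move to each raised path point in one loop, without waiting for arrival.
; Fire spawns a projectile at the muzzle aimed at the target, then sets it up with the wisp and its ItemOwner component.
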(event Custom|Move
  (bind _returnvalue (Transformation|GetActorLocation))
  (bind _returnvalue_2 (Class|NavigationSystemV1|FindPathtoLocationSynchronously (Class|NavigationSystemV1|GetNavigationSystem) _returnvalue (.RandomLocation (Class|NavigationSystemV1|GetRandomPointinNavigableRadius _returnvalue 1e+03 0 0)) self 0))
  (for _array_element (Variables|/Script/NavigationSystem.NavigationPath|GetPathPoints _returnvalue_2)
    (AI|Navigation|SimpleMovetoLocation (Pawn|GetController) (+ _array_element "0, 0,400.000000"))))

(event EventBeginPlay
  (bind _staticmeshes (Variables|Default|GetStaticMeshes))
  (Components|StaticMesh|SetStaticMesh (Variables|Default|GetStaticMesh) (Utilities|Array|Get(acopy) _staticmeshes (Math|Random|RandomIntegerinRange 0 (- (Utilities|Array|Length _staticmeshes) 1)))))

(fn ConstructionScript
  (bind _staticmeshes (Variables|Default|GetStaticMeshes))
  (Utilities|Array|Add _staticmeshes "/Game/Users/Kacper/Wisp_Heads/Head.Head")
  (Utilities|Array|Add _staticmeshes "/Game/Users/Kacper/Wisp_Heads/Head2.Head2")
  (Utilities|Array|Add _staticmeshes "/Game/Users/Kacper/Wisp_Heads/Head3.Head3")
  (Utilities|Array|Add _staticmeshes "/Game/Users/Kacper/Wisp_Heads/Head4.Head4")
  (Utilities|Array|Add _staticmeshes "/Game/Users/Kacper/Wisp_Heads/Head5.Head5"))

(fn Fire
  (params (Fire%20At :type Actor%20Object%20Reference))
  (bind _muzzle (Variables|Default|GetMuzzle))
  (bind _returnvalue (Transformation|GetWorldLocation _muzzle))
  (bind _returnvalue_2 (Game|SpawnActorfromClass (Variables|Default|GetProjectile) (Math|Transform|MakeTransform _returnvalue (Math|Rotator|FindLookatRotation _returnvalue (Transformation|GetActorLocation Fire%20At))) "Undefined" 0 0))
  (Class|Projectile|SetupProjectile _returnvalue_2 self (Variables|Default|GetItemOwner))
  (return true))