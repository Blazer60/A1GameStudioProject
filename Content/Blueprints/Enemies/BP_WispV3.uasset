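; BP_WispV3 is a wisp enemy Blueprint that extends a parent class with a randomized look and a delayed attack.
; On BeginPlay it runs the parent logic, then sets the WispHead mesh to a random entry from its StaticMeshes array.
; Its Fire event waits two seconds before passing the target to the parent's Fire.
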(event EventBeginPlay
  (bind _staticmeshes (Variables|Default|GetStaticMeshes))
  (|CallParentFunction)
  (Components|StaticMesh|SetStaticMesh (Variables|Default|GetWisp%20Head) (Utilities|Array|Get(acopy) _staticmeshes (Math|Random|RandomIntegerinRange 0 (Utilities|Array|LastIndex _staticmeshes)))))

(event EventFire
  (params (Fire%20At :type Actor%20Object%20Reference))
  (Utilities|FlowControl|Delay 2.0)
  (|CallParentFunction Fire%20At))

(fn ConstructionScript
  (|CallParentFunction))