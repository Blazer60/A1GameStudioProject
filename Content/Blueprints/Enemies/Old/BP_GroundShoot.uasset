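; BP_GroundShoot is an enemy shooting actor that launches a projectile at a target actor.
; Fire spawns the Projectile class at the Muzzle location, rotated to face the target's location at that moment.
; It then passes itself and its ItemOwner to the projectile's SetupProjectile and always returns true.
; The event graph and construction script are empty, so firing depends on an external call.
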(event EventBeginPlay)

(event Collision|EventActorBeginOverlap
  (params (OtherActor :type Actor%20Object%20Reference)))

(event EventTick
  (params (DeltaSeconds :type Float%20%28single-precision%29)))

(fn ConstructionScript)

(fn Fire
  (params (Fire%20At :type Actor%20Object%20Reference))
  (bind _muzzle (Variables|Default|GetMuzzle))
  (bind _returnvalue (Transformation|GetWorldLocation _muzzle))
  (bind _returnvalue_2 (Game|SpawnActorfromClass (Variables|Default|GetProjectile) (Math|Transform|MakeTransform _returnvalue (Math|Rotator|FindLookatRotation _returnvalue (Transformation|GetActorLocation Fire%20At))) "Undefined" 0 0))
  (Class|Projectile|SetupProjectile _returnvalue_2 self (Variables|Default|GetItemOwner))
  (return true))