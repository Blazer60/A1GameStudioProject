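; BP_SceneDirector is a gameplay-rules Blueprint that scatters loot chests around the level through its SpawnChest event.
; It picks a random navigable point around the navmesh-projected world origin, reprojects it vertically, and spawns the given chest class there with random yaw.
; Spawns that cannot avoid collision are skipped.
; Successful ones are lowered slightly and set up with an item and rarity drawn randomly from the Items array.
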(event EventBeginPlay)

(event Collision|EventActorBeginOverlap
  (params (OtherActor :type Actor%20Object%20Reference)))

(event EventTick
  (params (DeltaSeconds :type Float%20%28single-precision%29)))

(event EventSpawnChest
  (params (Chest :type Chest%20Class%20Reference))
  (bind _items (Variables|Default|GetItems))
  (bind _items_2 (Variables|Default|GetItems))
  (bind _returnvalue (Utilities|Array|LastIndex _items))
  (bind _returnvalue_2 (Math|Random|RandomIntegerinRange 0 _returnvalue))
  (bind _output (Utilities|Array|Get(acopy) _items_2 _returnvalue_2))
  (bind _returnvalue_3 (Game|SpawnActorfromClass Chest (Math|Transform|MakeTransform (.ProjectedLocation (AI|Navigation|ProjectPointtoNavigation (.RandomLocation (Class|NavigationSystemV1|GetRandomPointinNavigableRadius (.ProjectedLocation (AI|Navigation|ProjectPointtoNavigation (Math|Vector|VectorZero) 0 0 "500.000000,500.000000,100000.000000")) 8e+03 0 0)) 0 0 "0, 0,100000.000000")) (Math|Rotator|MakeRotator 0.0 0.0 (Math|Random|RandomFloatinRange 0.0 359.0))) "AdjustIfPossibleButDontSpawnIfColliding" 0 0))
  (Utilities|IsValid _returnvalue_3
    (:Is%20Valid
      (Transformation|SetActorLocation _returnvalue_3 (+ (Transformation|GetActorLocation _returnvalue_3) "0, 0,-15.000000") false false)
      (Class|Chest|Setup _returnvalue_3 (Variables|/Script/A1GameStudioProject.ItemDetails|GetWorldItem _output) (Variables|/Script/A1GameStudioProject.ItemDetails|GetRarity _output)))))

(fn ConstructionScript)