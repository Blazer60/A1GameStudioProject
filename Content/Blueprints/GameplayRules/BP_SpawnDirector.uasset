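; Spawn director that places groups of enemies in a ranged zone around the first player's pawn, which it caches on BeginPlay.
; SpawnEnemy picks a group center from the enemy details, then scatters each member on navigable points within the group's coherence radius.
; Spawns with an ItemOwner component are leveled up via EnemyLevel and given the supplied items.
; Nothing in this graph triggers spawning; SpawnEnemy relies on an external call.
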(event EventBeginPlay
  (Variables|Default|SetTracking (Game|Player|GetPlayerPawn 0)))

(event Collision|EventActorBeginOverlap
  (params (OtherActor :type Actor%20Object%20Reference)))

(event EventTick
  (params (DeltaSeconds :type Float%20%28single-precision%29)))

(event EventSpawnEnemy
  (params (EnemyDetails :type Enemy%20Details%20Object%20Reference) (EnemyItems :type Array%20of%20Item%20Details%20Object%20References))
  (Variables|Default|SetLocation (+ (Transformation|GetActorLocation (Variables|Default|GetTracking)) (Class|SpawnDirector|GetRandomPointinZone (Variables|/Script/A1GameStudioProject.EnemyDetails|GetMinRange EnemyDetails) (Variables|/Script/A1GameStudioProject.EnemyDetails|GetMaxRange EnemyDetails))))
  (for _index (range 1 (Variables|/Script/A1GameStudioProject.EnemyDetails|GetGroupSize EnemyDetails))
    (bind _returnvalue (Game|SpawnActorfromClass (Variables|/Script/A1GameStudioProject.EnemyDetails|GetToSpawn EnemyDetails) (Math|Transform|MakeTransform (.RandomLocation (Class|NavigationSystemV1|GetRandomPointinNavigableRadius (Variables|Default|GetLocation) (Variables|/Script/A1GameStudioProject.EnemyDetails|GetGroupCoherence EnemyDetails) 0 0))) "Undefined" 0 0))
    (if (Utilities|IsValid (Actor|GetComponentbyClass _returnvalue "/Script/A1GameStudioProject.ItemOwner"))
      (Class|ItemOwner|LevelUp (Actor|GetComponentbyClass _returnvalue "/Script/A1GameStudioProject.ItemOwner") (Class|SpawnDirector|EnemyLevel))
      (for _array_element EnemyItems
        (Class|ItemOwner|AddItem (Actor|GetComponentbyClass _returnvalue "/Script/A1GameStudioProject.ItemOwner") (Variables|/Script/A1GameStudioProject.ItemDetails|GetItemComponent _array_element) (Variables|/Script/A1GameStudioProject.ItemDetails|GetQuantity _array_element))))))

(fn ConstructionScript)