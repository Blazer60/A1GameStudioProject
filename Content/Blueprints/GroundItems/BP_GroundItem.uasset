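; BP_GroundItem is a pickup actor that places an item in the world for an overlapping actor to collect.
; When its collision is overlapped by an actor with an ItemOwner component, it adds its item class and quantity to that owner and destroys itself.
; A disconnected older branch, which increases an existing item component or adds and attaches a new one, remains in the graph but never runs.
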(event OnComponentBeginOverlap(Collision)
  (params (OverlappedComponent :type Primitive%20Component%20Object%20Reference) (OtherActor :type Actor%20Object%20Reference) (OtherComp :type Primitive%20Component%20Object%20Reference) (OtherBodyIndex :type Integer) (bFromSweep :type Boolean) (SweepResult :type Hit%20Result%20Structure%20%28by%20ref%29))
  (bind _returnvalue (Actor|GetComponentbyClass OtherActor "/Script/A1GameStudioProject.ItemOwner"))
  (if (Utilities|IsValid _returnvalue)
    (Class|ItemOwner|AddItem _returnvalue (Variables|Default|GetItem%20Component) (Variables|Default|GetQuantity))
    (Actor|DestroyActor)))

(fn ConstructionScript)