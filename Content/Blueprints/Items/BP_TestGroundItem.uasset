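; BP_TestGroundItem is a test ground pickup that grants an item component to an actor overlapping its sphere.
; It only acts on actors with an ItemOwner component, increasing an existing ItemType component or adding one through ItemOwner and calling OnAttach, then destroys itself.
; The item class comes from ItemType, replacing an unused legacy branch hard-wired to BP_TestItem.
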(event OnComponentBeginOverlap(Sphere)
  (params (OverlappedComponent :type Primitive%20Component%20Object%20Reference) (OtherActor :type Actor%20Object%20Reference) (OtherComp :type Primitive%20Component%20Object%20Reference) (OtherBodyIndex :type Integer) (bFromSweep :type Boolean) (SweepResult :type Hit%20Result%20Structure%20%28by%20ref%29))
  (bind _returnvalue (Actor|GetComponentbyClass OtherActor "/Script/A1GameStudioProject.ItemOwner"))
  (bind _item_type (Variables|Default|GetItem%20Type))
  (bind _returnvalue_2 (Actor|GetComponentbyClass OtherActor _item_type))
  (if (Utilities|IsValid _returnvalue)
    (if (Utilities|IsValid _returnvalue_2)
      (Class|ItemComponent|OnIncrease _returnvalue_2)
      (else
        (bind _returnvalue_3 (Class|ItemOwner|AddItem _returnvalue (Variables|Default|GetItem%20Type)))
        (Class|ItemComponent|OnAttach _returnvalue_3)))
    (Actor|DestroyActor)))

(fn ConstructionScript)