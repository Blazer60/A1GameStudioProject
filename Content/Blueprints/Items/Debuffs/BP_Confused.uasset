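; BP_Confused is a debuff item that confuses its owner by temporarily switching which side it is on.
; On attach it stores the owner's original Type, then flips Player to Enemy and anything else to Player.
; It also spawns confusion-symbol particles on the owner's BP_DebuffEmitterLocation component, if one exists.
; On detach it restores the original Type and destroys the particle component.
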(event EventBeginPlay)

(event EventTick
  (params (DeltaSeconds :type Float%20%28single-precision%29)))

(event EventOnAttach
  (bind _returnvalue (Class|ItemComponent|ItemOwner))
  (bind _returnvalue_2 (Components|GetOwner))
  (bind _returnvalue_3 (Actor|GetComponentbyClass _returnvalue_2 "/Game/Blueprints/BP_DebuffEmitterLocation.BP_DebuffEmitterLocation_C"))
  (Variables|Default|SetOriginal%20Type (Variables|/Script/A1GameStudioProject.ItemOwner|GetType (Class|ItemComponent|ItemOwner)))
  (if (Utilities|Enum|Equal(Enum) (Variables|/Script/A1GameStudioProject.ItemOwner|GetType (Class|ItemComponent|ItemOwner)) "Player")
    (Variables|/Script/A1GameStudioProject.ItemOwner|SetType _returnvalue "Enemy")
    (else
      (Variables|/Script/A1GameStudioProject.ItemOwner|SetType _returnvalue "Player")))
  (Utilities|IsValid _returnvalue_3
    (:Is%20Valid
      (bind _returnvalue_4 (Effects|SpawnEmitterAttached "/Game/Users/Luke/ParticleSystemWIP/DebuffSymbols/P_ConfusionSymbols.P_ConfusionSymbols" _returnvalue_3 "None"))
      (Variables|Default|SetParticleSystem _returnvalue_4))))

(event EventOnDetach
  (Variables|/Script/A1GameStudioProject.ItemOwner|SetType (Class|ItemComponent|ItemOwner) (Variables|Default|GetOriginal%20Type))
  (Components|DestroyComponent (Variables|Default|GetParticleSystem))
  (Variables|Default|SetParticleSystem 0))