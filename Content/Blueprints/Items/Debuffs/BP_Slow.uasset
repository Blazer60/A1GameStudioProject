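; BP_Slow is a debuff item that reduces its owner's speed while attached.
; On attach it takes a fraction of the owner's total speed, stores it, and subtracts it from the additional speed modifier.
; It also spawns a slow-symbol particle emitter on the owner's debuff emitter location component, if one exists.
; On detach it restores the stored amount and destroys the particles.
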(event EventBeginPlay)

(event EventTick
  (params (DeltaSeconds :type Float%20%28single-precision%29)))

(event EventOnAttach
  (bind _returnvalue (Class|ItemComponent|ItemOwner))
  (bind _returnvalue_2 (Components|GetOwner))
  (bind _returnvalue_3 (Actor|GetComponentbyClass _returnvalue_2 "/Game/Blueprints/BP_DebuffEmitterLocation.BP_DebuffEmitterLocation_C"))
  (bind _speed (Variables|/Script/A1GameStudioProject.ItemOwner|GetSpeed _returnvalue))
  (bind _output_get (Variables|Default|SetSpeed%20Decrease (* (Class|Stat|Total _speed) (Variables|Default|GetReduction%20Multiplier))))
  (Variables|/Script/A1GameStudioProject.Stat|SetAdditional _speed (- (Variables|/Script/A1GameStudioProject.Stat|GetAdditional _speed) _output_get))
  (Utilities|IsValid _returnvalue_3
    (:Is%20Valid
      (bind _returnvalue_4 (Effects|SpawnEmitterAttached "/Game/Users/Luke/ParticleSystemWIP/DebuffSymbols/P_SlowSymbols.P_SlowSymbols" _returnvalue_3 "None"))
      (Variables|Default|SetParticleSystem _returnvalue_4))))

(event EventOnDetach
  (bind _returnvalue (Class|ItemComponent|ItemOwner))
  (bind _speed (Variables|/Script/A1GameStudioProject.ItemOwner|GetSpeed _returnvalue))
  (Variables|/Script/A1GameStudioProject.Stat|SetAdditional _speed (+ (Variables|Default|GetSpeed%20Decrease) (Variables|/Script/A1GameStudioProject.Stat|GetAdditional _speed)))
  (Components|DestroyComponent (Variables|Default|GetParticleSystem))
  (Variables|Default|SetParticleSystem 0))

(event EventOnDecrease)