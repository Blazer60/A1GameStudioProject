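; BP_GroundShooterProjectile is a projectile actor that accelerates forward while spinning and destroys itself on impact.
; Each tick it applies a mass-independent force along the SphereComponent's forward vector, scaled by Force and delta time.
; The same tick rolls the Scene component at RotationRate for the spin.
; A hit event or the ProjectileMovementComponent stopping destroys the actor.
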(event OnProjectileStop(ProjectileMovementComponent)
  (params (ImpactResult :type Hit%20Result%20Structure%20%28by%20ref%29))
  (Actor|DestroyActor))

(event EventBeginPlay)

(event Collision|EventActorBeginOverlap
  (params (OtherActor :type Actor%20Object%20Reference)))

(event EventTick
  (params (DeltaSeconds :type Float%20%28single-precision%29))
  (Physics|AddForce (Variables|Default|GetSphereComponent) (* (Math|Vector|GetForwardVector (Variables|Default|GetSphereComponent)) (* (Variables|Default|GetForce) DeltaSeconds)) "None" true)
  (Transformation|AddRelativeRotation (Variables|Default|GetScene) (Math|Rotator|MakeRotator (* DeltaSeconds (Variables|Default|GetRotationRate)) 0.0 0.0) false false))

(event EventOnHit
  (params (OtherOwner :type Item%20Owner%20Object%20Reference) (Location :type Vector :default "0, 0, 0"))
  (Actor|DestroyActor))

(fn ConstructionScript)