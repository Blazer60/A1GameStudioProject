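; BP_ArcSpawnShot is a projectile prop that delivers an item, spawning it where the shot comes to a stop.
; Setup stores the item class and rarity, then picks a flare particle template for the trail to match Common, Uncommon or Rare.
; When projectile movement stops, it spawns the item at the impact location and destroys itself after a short delay.
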(event OnProjectileStop(ProjectileMovement)
  (params (ImpactResult :type Hit%20Result%20Structure%20%28by%20ref%29))
  (Game|SpawnActorfromClass (Variables|Default|GetItem) (Math|Conversions|ToTransform(Vector) (.Location (Collision|BreakHitResult ImpactResult))) "Undefined" 0 0)
  (Utilities|FlowControl|Delay 0.4)
  (Actor|DestroyActor))

(event Custom|Setup
  (params (Item :type World%20Item%20Class%20Reference) (Rarity :type ERarity%20Enum :default "Common"))
  (bind _trail (Variables|Default|GetTrail))
  (Variables|Default|SetItem Item)
  (bind _output_get (Variables|Default|SetRarity Rarity))
  (switch Utilities|FlowControl|Switch|SwitchonERarity _output_get
    (:Common
      (Effects|Components|ParticleSystem|SetTemplate _trail "/Game/Users/Luke/ParticleSystemWIP/ItemFlare/P_Flare_Common.P_Flare_Common"))
    (:Uncommon
      (Effects|Components|ParticleSystem|SetTemplate _trail "/Game/Users/Luke/ParticleSystemWIP/ItemFlare/P_Flare_Uncommon.P_Flare_Uncommon"))
    (:Rare
      (Effects|Components|ParticleSystem|SetTemplate _trail "/Game/Users/Luke/ParticleSystemWIP/ItemFlare/P_Flare_Rare.P_Flare_Rare"))))

(event EventBeginPlay)

(event Collision|EventActorBeginOverlap
  (params (OtherActor :type Actor%20Object%20Reference)))

(event EventTick
  (params (DeltaSeconds :type Float%20%28single-precision%29)))

(fn ConstructionScript)