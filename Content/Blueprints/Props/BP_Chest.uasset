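; Interactable chest prop that slides two lids apart and launches its loot item.
; Player overlap toggles a prompt widget, and Interact opens the chest once.
; Opening plays a Niagara burst, sound and lid timeline, then spawns a BP_ArcSpawnShot set up with Item and Rarity.
; A chest without an item opens itself shortly after BeginPlay and spawns nothing when finished.
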(event OnComponentEndOverlap(InteractCollision)
  (params (OverlappedComponent :type Primitive%20Component%20Object%20Reference) (OtherActor :type Actor%20Object%20Reference) (OtherComp :type Primitive%20Component%20Object%20Reference) (OtherBodyIndex :type Integer))
  (if (== OtherActor (Game|Player|GetPlayerPawn 0))
    (CallFunction|HideInteractUI)))

(event OnComponentBeginOverlap(InteractCollision)
  (params (OverlappedComponent :type Primitive%20Component%20Object%20Reference) (OtherActor :type Actor%20Object%20Reference) (OtherComp :type Primitive%20Component%20Object%20Reference) (OtherBodyIndex :type Integer) (bFromSweep :type Boolean) (SweepResult :type Hit%20Result%20Structure%20%28by%20ref%29))
  (if (== OtherActor (Game|Player|GetPlayerPawn 0))
    (CallFunction|ShowInteractUI)))

(event Custom|PlayTimeline
  (Niagara|SpawnSystematLocation "/Game/Users/Luke/ParticleSystemWIP/StylisedExplosion/Explosion_NS.Explosion_NS" (Transformation|GetWorldLocation (Variables|Default|GetProjectileSpawnPoint)))
  (Audio|PlaySoundatLocation "/Game/Users/Lauren/Audio/Misc/ChestOpening.ChestOpening" "0, 0, 0" "0, 0, 0" 1.0 1.0 0.0 0 0 0)
  (bind _offset (Timeline|Timer Play)
    (:Update
      (Transformation|SetRelativeLocation (Variables|Default|GetLeft) (+ (Variables|Default|GetLeftLidStartingPosition) (Math|Vector|MakeVector (* _offset (Variables|Default|GetDistance) -1.0) 0.0 0.0)) false false)
      (Transformation|SetRelativeLocation (Variables|Default|GetRight) (+ (Variables|Default|GetRightLidStartingPosition) (Math|Vector|MakeVector (* _offset (Variables|Default|GetDistance) 1.0) 0.0 0.0)) false false))
    (:Finished
      (CallFunction|SpawnProjectile))))

(event Custom|SpawnProjectile
  (if (Utilities|IsValidClass (Variables|Default|GetItem))
    (bind _returnvalue (Game|SpawnActorfromClass "/Game/Blueprints/Props/BP_ArcSpawnShot.BP_ArcSpawnShot_C" (Transformation|GetWorldTransform (Variables|Default|GetProjectileSpawnPoint)) "Undefined" 0 0))
    (Default|Setup _returnvalue (Variables|Default|GetItem) (Variables|Default|GetRarity))))

(event EventBeginPlay
  (Variables|Default|SetLeftLidStartingPosition (Variables|/Script/Engine.SceneComponent|GetRelativeLocation (Variables|Default|GetLeft)))
  (Variables|Default|SetRightLidStartingPosition (Variables|/Script/Engine.SceneComponent|GetRelativeLocation (Variables|Default|GetRight)))
  (Utilities|FlowControl|Delay 1.0)
  (if (not (Utilities|IsValidClass (Variables|Default|GetItem)))
    (Variables|Default|SetIsOpened? true)
    (CallFunction|PlayTimeline)))

(event EventShowInteractUI
  (if (not (or (Variables|Default|GetIsOpened?) (Variables|Default|GetIsShowingUI?)))
    (bind _returnvalue (UserInterface|CreateWidget "/Game/ChestBP/Interact_Prompt_Widget.Interact_Prompt_Widget_C"))
    (bind _output_get (Variables|Default|SetInteractWidget _returnvalue))
    (UserInterface|Viewport|AddtoViewport _output_get 0)
    (Variables|Default|SetIsShowingUI? true)))

(event EventHideInteractUI
  (if (and (Variables|Default|GetIsShowingUI?) (Utilities|IsValid (Variables|Default|GetInteractWidget)))
    (Widget|RemovefromParent (Variables|Default|GetInteractWidget))
    (Variables|Default|SetIsShowingUI? false)))

(fn ConstructionScript)

(fn CanbeInteracted?
  (return (and (not (Variables|Default|GetIsOpened?)) (Utilities|IsValidClass (Variables|Default|GetItem)))))

(fn Interact
  (params (Interactor :type Character%20Object%20Reference))
  (bind _interactwidget (Variables|Default|GetInteractWidget))
  (if (Variables|Default|GetIsOpened?)
    (return false)
    (else
      (Variables|Default|SetIsOpened? true)
      (Utilities|IsValid _interactwidget
        (:Is%20Valid
          (Variables|/Game/ChestBP/Interact_Prompt_Widget.Interact_Prompt_Widget_C|SetIsPressed _interactwidget true)
          (Variables|/Game/ChestBP/Interact_Prompt_Widget.Interact_Prompt_Widget_C|SetIsPressed _interactwidget false)
          (Widget|RemovefromParent _interactwidget))
        (:Is%20Not%20Valid
          _))
      (CallFunction|PlayTimeline)
      (return true))))