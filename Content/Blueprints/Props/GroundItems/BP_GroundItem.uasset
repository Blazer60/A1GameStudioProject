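; BP_GroundItem is a world pickup that grants an item and quantity to overlapping actors that have an ItemOwner component.
; On overlap it calls AddItem on that component, destroys itself and plays an equip sound at its location.
; A spawn sound plays shortly after BeginPlay.
; The construction script sets the RarityBand material to match the Common, Uncommon or Rare rarity.
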(event OnComponentBeginOverlap(Collision)
  (params (OverlappedComponent :type Primitive%20Component%20Object%20Reference) (OtherActor :type Actor%20Object%20Reference) (OtherComp :type Primitive%20Component%20Object%20Reference) (OtherBodyIndex :type Integer) (bFromSweep :type Boolean) (SweepResult :type Hit%20Result%20Structure%20%28by%20ref%29))
  (bind _returnvalue (Actor|GetComponentbyClass OtherActor "/Script/A1GameStudioProject.ItemOwner"))
  (if (Utilities|IsValid _returnvalue)
    (Class|ItemOwner|AddItem _returnvalue (Variables|Default|GetItem) (Variables|Default|GetQuantity))
    (Actor|DestroyActor)
    (Audio|PlaySoundatLocation "/Game/Users/Lauren/Audio/Items/ItemEquip_Cue.ItemEquip_Cue" (Transformation|GetActorLocation) "0, 0, 0" 1.0 1.0 0.0 0 0 0)))

(event EventBeginPlay
  (Utilities|FlowControl|Delay 0.2)
  (Audio|PlaySoundatLocation (Variables|Default|GetSpawnSound) (Transformation|GetActorLocation) "0, 0, 0" 1.0 1.0 0.0 0 0 0))

(fn ConstructionScript
  (Utilities|FlowControl|Sequence
    (:then_0
      (if (Utilities|Enum|Equal(Enum) (Variables|Default|GetRarity) "Common")
        (Rendering|Material|SetMaterial (Variables|Default|GetRarityBand) 0 "/Game/Meshes/Materials/ItemRarity/M_RarityCommon.M_RarityCommon")))
    (:then_1
      (if (Utilities|Enum|Equal(Enum) (Variables|Default|GetRarity) "Uncommon")
        (Rendering|Material|SetMaterial (Variables|Default|GetRarityBand) 0 "/Game/Meshes/Materials/ItemRarity/M_RarityUncommon.M_RarityUncommon")))
    (:then_2
      (if (Utilities|Enum|Equal(Enum) (Variables|Default|GetRarity) "Rare")
        (Rendering|Material|SetMaterial (Variables|Default|GetRarityBand) 0 "/Game/Meshes/Materials/ItemRarity/M_RarityRare.M_RarityRare")))))