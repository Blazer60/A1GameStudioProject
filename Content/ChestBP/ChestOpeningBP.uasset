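; An interactable chest that opens once through Interact, playing a coin particle burst.
; ShowInteractUI creates a prompt widget and opens a gate; HideInteractUI, or the player leaving the lid's overlap, removes it and closes the gate.
; OpenChest sets IsOpened before the gate, which passes to a timeline that rotates an Arrow component, spawns coins every update and removes the prompt after a delay.
; Begin overlap only casts to the player.
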(event OnComponentEndOverlap(ChestLid)
  (params (OverlappedComponent :type Primitive%20Component%20Object%20Reference) (OtherActor :type Actor%20Object%20Reference) (OtherComp :type Primitive%20Component%20Object%20Reference) (OtherBodyIndex :type Integer))
  (Utilities|Casting|CastToBP_MainPlayer OtherActor)
  (if (Variables|Default|GetisShowingUI)
    (Utilities|IsValid (stale EventShowInteractUI _returnvalue)
      (:Is%20Valid
        (Widget|RemovefromParent (stale EventShowInteractUI _returnvalue))
        (Variables|Default|SetisShowingUI false)
        (Utilities|FlowControl|Gate true) ; enters at Close
      ))))

(event OnComponentBeginOverlap(ChestLid)
  (params (OverlappedComponent :type Primitive%20Component%20Object%20Reference) (OtherActor :type Actor%20Object%20Reference) (OtherComp :type Primitive%20Component%20Object%20Reference) (OtherBodyIndex :type Integer) (bFromSweep :type Boolean) (SweepResult :type Hit%20Result%20Structure%20%28by%20ref%29))
  (Utilities|Casting|CastToBP_MainPlayer OtherActor))

(event Custom|Open%20Chest
  (if (not (Variables|Default|GetisOpened))
    (Variables|Default|SetisOpened true)
    (Variables|/Game/ChestBP/Interact_Prompt_Widget.Interact_Prompt_Widget_C|SetIsPressed (stale EventShowInteractUI _returnvalue) true)
    (Variables|/Game/ChestBP/Interact_Prompt_Widget.Interact_Prompt_Widget_C|SetIsPressed (stale EventShowInteractUI _returnvalue) false)
    (Utilities|FlowControl|Gate true
      (:Exit
        (bind _newtrack_0 (Timeline|Timeline_0 Play)
          (:Update
            (Effects|SpawnEmitteratLocation "/Game/ParticleSystems/CoinShower/CoinsNoLoop_P.CoinsNoLoop_P" (Transformation|GetWorldLocation (Variables|Default|GetChestLid)))
            (Transformation|SetRelativeRotation (Variables|Default|GetArrow) (Math|Rotator|MakeRotator (* _newtrack_0 (Variables|Default|GetAngle)) 0.0 0.0) false false)
            (Utilities|FlowControl|Delay 0.2)
            (Widget|RemovefromParent (stale EventShowInteractUI _returnvalue))))))))

(event EventShowInteractUI
  (if (not (Variables|Default|GetisShowingUI))
    (if (not (Variables|Default|GetisOpened))
      (bind _returnvalue (UserInterface|CreateWidget "/Game/ChestBP/Interact_Prompt_Widget.Interact_Prompt_Widget_C"))
      (UserInterface|Viewport|AddtoViewport _returnvalue 0)
      (Variables|Default|SetisShowingUI true)
      (Utilities|FlowControl|Gate true) ; enters at Open
    )))

(event EventHideInteractUI
  (if (Variables|Default|GetisShowingUI)
    (Utilities|IsValid (stale EventShowInteractUI _returnvalue)
      (:Is%20Valid
        (Widget|RemovefromParent (stale EventShowInteractUI _returnvalue))
        (Variables|Default|SetisShowingUI false)
        (Utilities|FlowControl|Gate true) ; enters at Close
      ))))

(fn ConstructionScript)

(fn CanbeInteracted?
  (return (not (Variables|Default|GetisOpened))))

(fn Interact
  (params (Interactor :type Character%20Object%20Reference))
  (CallFunction|OpenChest)
  (return true))