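; Killer Queen master Blueprint, whose Arrow component hovers up and down while turning to face the player.
; Each tick it casts the player pawn to BP_MainPlayer, then interpolates the Arrow's world rotation from the actor's rotation toward a look-at rotation.
; A sine of time since creation then offsets the Arrow's Z from the relative location cached at BeginPlay, scaled by float distance and speed.
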(event Custom|Face%20Player
  ;[1 1 1] Smooth transition from arrow rotation to face the player (DELETED: then repeat)
  (Transformation|SetWorldRotation (Variables|Default|GetArrow) (Math|Interpolation|RInterpTo (Transformation|GetActorRotation) (Math|Rotator|FindLookatRotation (Transformation|GetWorldLocation (Variables|Default|GetArrow)) (Transformation|GetActorLocation (Variables|Default|GetChar%20Ref))) (Utilities|Time|GetWorldDeltaSeconds) 2e+02) false false))

(event EventTick
  (params (DeltaSeconds :type Float%20%28single-precision%29))
  (bind _killer_queen_relative_location (Variables|Default|GetKiller_Queen%20Relative%20Location))
  (Utilities|FlowControl|Sequence
    (:then_0
      ;[1 1 1] Sets the player as the Char Ref then begins Face Player Event
      (bind _asbp_main_player (Utilities|Casting|CastToBP_MainPlayer (Game|Player|GetPlayerPawn 0)))
      (Variables|Default|SetChar%20Ref _asbp_main_player)
      (CallFunction|FacePlayer))
    (:then_1
      (Transformation|SetRelativeLocation (Variables|Default|GetArrow) (Math|Vector|MakeVector (.x _killer_queen_relative_location) (.y _killer_queen_relative_location) (+ (.z _killer_queen_relative_location) (* (Variables|Default|GetFloat%20Distance) (Math|Trig|Sin(Degrees) (* (Actor|GetGameTimeSinceCreation) (Variables|Default|GetFloat%20Speed)))))) false false))))

(event EventBeginPlay
  (Variables|Default|SetKiller_Queen%20Relative%20Location (Variables|/Script/Engine.SceneComponent|GetRelativeLocation (Variables|Default|GetArrow))))

(fn ConstructionScript)